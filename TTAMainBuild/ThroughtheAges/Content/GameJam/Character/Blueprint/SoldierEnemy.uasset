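; SoldierEnemy is an enemy character that shows a text label, apparently a Q/W/E/R key prompt, chosen by its position.
; Each Tick, until Set is true, it matches the capsule's truncated world Y against four fixed lane positions and assigns the corresponding text to Q.
; Only the R1 branch sets the flag, after which Tick just keeps making the label visible.
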(event EventTick
  (params (DeltaSeconds :type Float%20%28single-precision%29))
  (if (Variables|Default|Getset?)
    (if true
      (Rendering|SetVisibility (Variables|Default|GetQ) true false))
    (elif (== (Math|Float|Truncate (.Y (Math|Vector|BreakVector (Transformation|GetWorldLocation (Variables|Collision|GetCapsuleComponent))))) -1500)
      (Rendering|Components|TextRender|SetText (Variables|Default|GetQ) (Variables|Default|Getq1))
      (elif (== (Math|Float|Truncate (.Y (Math|Vector|BreakVector (Transformation|GetWorldLocation (Variables|Collision|GetCapsuleComponent))))) -1300)
        (Rendering|Components|TextRender|SetText (Variables|Default|GetQ) (Variables|Default|Getw1))
        (elif (== (Math|Float|Truncate (.Y (Math|Vector|BreakVector (Transformation|GetWorldLocation (Variables|Collision|GetCapsuleComponent))))) -1100)
          (Rendering|Components|TextRender|SetText (Variables|Default|GetQ) (Variables|Default|Gete1))
          (elif (== (Math|Float|Truncate (.Y (Math|Vector|BreakVector (Transformation|GetWorldLocation (Variables|Collision|GetCapsuleComponent))))) -900)
            (Rendering|Components|TextRender|SetText (Variables|Default|GetQ) (Variables|Default|Getr1))
            (Variables|Default|Setset? true)))))))

(fn ConstructionScript)